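; Geometry collection wall actor that reacts to Chaos destruction with Niagara effects.
; Chaos collisions spawn a collision effect oriented to the impact normal, but only when the other component belongs to the sports car pawn.
; Break and removal events spawn destruction and disappear effects at their locations.
; Tick accumulates a Timer variable that nothing in this Blueprint reads.
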(event OnChaosBreakEvent(GeometryCollectionComponent)
  (params (BreakEvent :type Chaos%20Break%20Event%20Structure%20%28by%20ref%29))
  (bind (_component _location _orientation) (Utilities|Struct|BreakChaosBreakEvent BreakEvent))
  (Niagara|SpawnSystematLocation "/Game/Chaos/Niagara/NS_Destruction.NS_Destruction" _location (Class|KismetMathLibrary|QuatRotator _orientation)))

(event OnChaosRemovalEvent(GeometryCollectionComponent)
  (params (RemovalEvent :type Chaos%20Removal%20Event%20Structure%20%28by%20ref%29))
  (Niagara|SpawnSystematLocation "/Game/Chaos/Niagara/NS_Disapear.NS_Disapear" (.Location (Utilities|Struct|BreakChaosRemovalEvent RemovalEvent))))

(event OnChaosPhysicsCollision(GeometryCollectionComponent)
  (params (CollisionInfo :type Chaos%20Physics%20Collision%20Info%20Structure%20%28by%20ref%29))
  (bind (_component _othercomponent _location _normal) (Utilities|Struct|BreakChaosPhysicsCollisionInfo CollisionInfo))
  (Utilities|Casting|CastToBP_SportsCar_Pawn (Components|GetOwner _othercomponent))
  (Niagara|SpawnSystematLocation "/Game/Chaos/Niagara/NS_Collision.NS_Collision" _location (Math|Conversions|RotationFromXVector _normal)))

(event EventBeginPlay)

(event Collision|EventActorBeginOverlap
  (params (OtherActor :type Actor%20Object%20Reference)))

(event EventTick
  (params (DeltaSeconds :type Float%20%28single-precision%29))
  (Variables|Default|SetTimer (+ DeltaSeconds (Variables|Default|GetTimer))))

(fn ConstructionScript)